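; BP_Champion is a lottery simulator for Daletou and Shuangseqiu that counts draws until a target prize tier is hit.
; DoRandom draws red and blue balls without replacement, sorts them and sends them to the PanelVaria widget.
; Position-by-position comparison with the panel's winning numbers yields hit counts for per-game tier rules.
; Wins stop the run and optionally update average attempts and odds; RandomBallNTime batch-writes draws to a path.
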(fn `CalculateAverageTimes`
  (params (Array :type "Array of Integer"))
  (returns (ReturnValue :type Integer))
  (locals (LTemp :type Integer))
  (bind _ltemp (`local.LTemp`))
  (for _array_element Array
    (set `local.LTemp` (+ (`local.LTemp`) _array_element)))
  (set `self.PriceSimulateTotalNum` _ltemp)
  (return (/ _ltemp (`KismetArrayLibrary.Array_Length` Array))))

(fn `CheckHowMuchBallHit`
  (params (Simulate :type "Array of Integer") (Price :type "Array of Integer") (Type :type "/Game/Blueprints/ChampionType Enum" :default "NewEnumerator0"))
  (returns (RedTimes :type Integer) (BlueTiems :type Integer) (PositionResult :type "Array of Boolean"))
  (locals (LForLoopTimes :type Integer) (LPositionResult :type "Array of Boolean") (LRedTimes :type Integer) (LBlueTimes :type Integer))
  (switch `/Game/Blueprints/ChampionType` Type
    (:`NewEnumerator0`
      (set `local.LForLoopTimes` 5))
    (:`NewEnumerator1`
      (set `local.LForLoopTimes` 6)))
  (for (_array_element _array_index) Simulate
    (if (< _array_index (`local.LForLoopTimes`))
      (bind _returnvalue (== _array_element (`|GetArrayItem` Price _array_index)))
      (`KismetArrayLibrary.Array_Add` (`local.LPositionResult`) _returnvalue)
      (if _returnvalue
        (`/Engine/EditorBlueprintResources/StandardMacros.IncrementInt` (`local.LRedTimes`)))
      (else
        (`KismetArrayLibrary.Array_Add` (`local.LPositionResult`) _returnvalue)
        (if _returnvalue
          (`/Engine/EditorBlueprintResources/StandardMacros.IncrementInt` (`local.LBlueTimes`))))))
  (return (`local.LRedTimes`) (`local.LBlueTimes`) (`local.LPositionResult`)))

(fn `CheckWinPriceLevelByExpect_DLT`
  (params (ExpectLevel :type Integer) (RedBallNum :type Integer) (BlueBallNum :type Integer))
  (returns (WinPriceLevel :type Integer))
  (locals (LExpectLevel :type Integer) (LRedBall :type Integer) (LBlueBall :type Integer))
  (bind _lredball (`local.LRedBall`))
  (bind _lredball_2 (`local.LRedBall`))
  (bind _lblueball (`local.LBlueBall`))
  (bind _lredball_3 (`local.LRedBall`))
  (bind _lblueball_2 (`local.LBlueBall`))
  (bind _lblueball_3 (`local.LBlueBall`))
  (bind _lredball_4 (`local.LRedBall`))
  (bind _lblueball_4 (`local.LBlueBall`))
  (set `local.LExpectLevel` ExpectLevel)
  (set `local.LRedBall` RedBallNum)
  (set `local.LBlueBall` BlueBallNum)
  (`|ExecutionSequence`
    (:`then_0`
      (if (`self.DLT_1` _lredball_3 _lblueball_3)
        (return 1)))
    (:`then_1`
      (if (`self.DLT_2` _lredball_3 _lblueball_3)
        (if (>= (`local.LExpectLevel`) 2)
          (return 2))))
    (:`then_2`
      (if (`self.DLT_3` _lredball_4 _lblueball_4)
        (if (>= (`local.LExpectLevel`) 3)
          (return 3))))
    (:`then_3`
      (if (`self.DLT_4` _lredball_4 _lblueball_4)
        (if (>= (`local.LExpectLevel`) 4)
          (return 4))))
    (:`then_4`
      (if (`self.DLT_5` _lredball_2 _lblueball)
        (if (>= (`local.LExpectLevel`) 5)
          (return 5))))
    (:`then_5`
      (if (`self.DLT_6` _lredball_2 _lblueball)
        (if (>= (`local.LExpectLevel`) 6)
          (return 6))))
    (:`then_6`
      (if (`self.DLT_7` _lredball _lblueball_2)
        (if (>= (`local.LExpectLevel`) 7)
          (return 7))))
    (:`then_7`
      (if (`self.DLT_8` _lredball _lblueball_2)
        (if (>= (`local.LExpectLevel`) 8)
          (return 8))))
    (:`then_8`
      (if (`self.DLT_9` (`local.LRedBall`) (`local.LBlueBall`))
        (if (>= (`local.LExpectLevel`) 9)
          (return 9))))
    (:`then_9`
      (return 0))))

(fn `CheckWinPriceLevelByExpect_SSQ`
  (params (ExpectLevel :type Integer) (RedBallNum :type Integer) (BlueBallNum :type Integer))
  (returns (WinPriceLevel :type Integer))
  (locals (LExpectLevel :type Integer) (LRedBall :type Integer) (LBlueBall :type Integer))
  (bind _lredball (`local.LRedBall`))
  (bind _lblueball (`local.LBlueBall`))
  (bind _lredball_2 (`local.LRedBall`))
  (bind _lblueball_2 (`local.LBlueBall`))
  (bind _lredball_3 (`local.LRedBall`))
  (bind _lblueball_3 (`local.LBlueBall`))
  (set `local.LExpectLevel` ExpectLevel)
  (set `local.LRedBall` RedBallNum)
  (set `local.LBlueBall` BlueBallNum)
  (`|ExecutionSequence`
    (:`then_0`
      (if (`self.SSQ_1` _lredball_2 _lblueball_2)
        (return 1)))
    (:`then_1`
      (if (`self.SSQ_2` _lredball_2 _lblueball_2)
        (if (>= (`local.LExpectLevel`) 2)
          (return 2))))
    (:`then_2`
      (if (`self.SSQ_3` _lredball_3 _lblueball_3)
        (if (>= (`local.LExpectLevel`) 3)
          (return 3))))
    (:`then_3`
      (if (`self.SSQ_4` _lredball_3 _lblueball_3)
        (if (>= (`local.LExpectLevel`) 4)
          (return 4))))
    (:`then_4`
      (if (`self.SSQ_5` _lredball _lblueball)
        (if (>= (`local.LExpectLevel`) 5)
          (return 5))))
    (:`then_5`
      (if (`self.SSQ_6` _lredball _lblueball)
        (if (>= (`local.LExpectLevel`) 6)
          (return 6))))
    (:`then_6`
      (return 0))))

(fn `ClearAverageUIData`
  (`KismetArrayLibrary.Array_Clear` (`self.PriceTimesArray`))
  (set `self.PriceSimulateOrder` 0)
  (set `self.PriceAverageTimes` 0)
  (set `self.PriceSimulateTotalNum` 0)
  (set `self.WinPricePercent` 0.0)
  (`/Game/UI/WB_MainColorPanle.ResetAverageDatas` (`self.PanelVaria`)))

(fn `DoRandom`
  (locals (LTempResult :type "Array of Integer"))
  (bind _panelvaria (`self.PanelVaria`))
  (bind _ltempresult (`local.LTempResult`))
  (bind _panelvaria_2 (`self.PanelVaria`))
  (bind _pricetimesarray (`self.PriceTimesArray`))
  (`|ExecutionSequence`
    (:`then_0`
      ;[1 1 1] 计算每一注的红球和蓝球，并将它们记录下来
      (bind (_randomredballs _randomblueballs) (`self.Random Ball One Time`))
      (set `self.SortedRedBall` _randomredballs)
      (set `self.SortedBlueBall` _randomblueballs)
      (`KismetArrayLibrary.Array_Append` _ltempresult _randomredballs)
      (`KismetArrayLibrary.Array_Append` _ltempresult _randomblueballs))
    (:`then_1`
      (`/Game/UI/WB_MainColorPanle.FillBalls` (`self.PanelVaria`) (`self.SortedRedBall`) (`self.SortedBlueBall`)))
    (:`then_2`
      ;[1 1 1] 匹配奖项
      (`/Engine/EditorBlueprintResources/StandardMacros.IncrementInt` (`self.TempPriceMateTimes`)
        (:`  `
          (bind (_whetherprice _pricelevel _positionresult _hitrednum _hitbluenum) (`self.WhetherWinPrice` (`self.CurrentMode`) (`/Game/UI/WB_MainColorPanle.GetQiwangPrice` (`self.PanelVaria`)) (`local.LTempResult`)))
          (if _whetherprice
            ;;[0.04256 1 0] 匹配结果出来之后要做的事情
            (`|ExecutionSequence`
              (:`then_0`
                (set `self.RealPriceMateTimes` (`self.TempPriceMateTimes`))
                (set `self.TempPriceMateTimes` 0)
                ;;;[1 0.8872 0] 对平均次数进行处理
                (if (`/Game/UI/WB_MainColorPanle.GetWhetherRecordAverage` (`self.PanelVaria`))
                  (`KismetArrayLibrary.Array_Add` _pricetimesarray (`self.RealPriceMateTimes`))
                  (`self.CalculateAverageTimes` _pricetimesarray)
                  (set `self.WinPricePercent` (/ (`self.1Constance`) (`self.PriceAverageTimes`)))
                  (`/Engine/EditorBlueprintResources/StandardMacros.IncrementInt` (`self.PriceSimulateOrder`)
                    (:`  `
                      (`/Game/UI/WB_MainColorPanle.Add Expected Average Data` _panelvaria (`self.RealPriceMateTimes`) (`self.PriceSimulateOrder`))
                      (`Widget.SetVisibility` (`/Game/UI/WB_MainColorPanle.WB_ExpectAverage` _panelvaria) "SelfHitTestInvisible")))))
              (:`then_1`
                (`/Game/UI/WB_MainColorPanle.UpdateHitPriceUI` _panelvaria_2 _positionresult _hitrednum _hitbluenum _pricelevel)
                (`/Game/UI/WB_MainColorPanle.EventStop` _panelvaria_2)))))))))

(fn `InitBalls`
  (`|ExecutionSequence`
    (:`then_0`
      (for _index (range 1 (+ (`self.RedBallTotal`) 1))
        (`KismetArrayLibrary.Array_Add` (`self.RedBalls`) _index)))
    (:`then_1`
      (for _index_2 (range 1 (+ (`self.BlueBallTotal`) 1))
        (`KismetArrayLibrary.Array_Add` (`self.BlueBalls`) _index_2)))))

(fn `Jici`
  (locals (ResultArray :type "Array of Integer"))
  (`KismetArrayLibrary.Array_Append` (`local.ResultArray`) (`self.SortedRedBall`))
  (`KismetArrayLibrary.Array_Append` (`local.ResultArray`) (`self.SortedBlueBall`))
  (`/Game/UI/WB_MainColorPanle.Jici` (`self.PanelVaria`) (`self.CurrentMode`) (`local.ResultArray`)))

(fn `Random Ball One Time`
  (returns (RandomRedBalls :type "Array of Integer") (RandomBlueBalls :type "Array of Integer"))
  (locals (LRedRandom :type Integer) (LBlueRandom :type Integer))
  (bind _blueballs (`self.BlueBalls`))
  (bind _redballs (`self.RedBalls`))
  (`KismetArrayLibrary.Array_Clear` (`self.RandomRedBalls`))
  (`KismetArrayLibrary.Array_Clear` (`self.RandomBlueBalls`))
  (`KismetArrayLibrary.Array_Clear` (`self.RedBalls`))
  (`KismetArrayLibrary.Array_Clear` (`self.BlueBalls`))
  (`self.InitBalls`)
  (`|ExecutionSequence`
    (:`then_0`
      (for _ (range (`self.RedBallChoose`))
        (set `local.LRedRandom` (`KismetMathLibrary.RandomIntegerInRange` 0 (- (`KismetArrayLibrary.Array_Length` _redballs) 1)))
        (`KismetArrayLibrary.Array_Add` (`self.RandomRedBalls`) (`|GetArrayItem` _redballs (`local.LRedRandom`)))
        (`KismetArrayLibrary.Array_Remove` _redballs (`local.LRedRandom`))))
    (:`then_1`
      (for _ (range (`self.BlueBallChoose`))
        (set `local.LBlueRandom` (`KismetMathLibrary.RandomIntegerInRange` 0 (- (`KismetArrayLibrary.Array_Length` _blueballs) 1)))
        (`KismetArrayLibrary.Array_Add` (`self.RandomBlueBalls`) (`|GetArrayItem` _blueballs (`local.LBlueRandom`)))
        (`KismetArrayLibrary.Array_Remove` _blueballs (`local.LBlueRandom`))))
    (:`then_2`
      (return (`self.SortBall` (`self.RandomRedBalls`)) (`self.SortBall` (`self.RandomBlueBalls`))))))

(fn `RandomBallNTime`
  (params (N :type Integer) (Path :type String))
  (locals (LN :type Integer) (LResult :type "Array of Integer"))
  (bind _lresult (`local.LResult`))
  (set `local.LN` N)
  (for _ (range (`local.LN`))
    (bind (_randomredballs _randomblueballs) (`self.Random Ball One Time`))
    (`KismetArrayLibrary.Array_Append` _lresult _randomredballs)
    (`KismetArrayLibrary.Array_Append` _lresult _randomblueballs)
    (`BallFunctionLibrary.WriteBallResult` (`local.LResult`) Path)
    (`KismetArrayLibrary.Array_Clear` _lresult)))

(fn `SortBall`
  (params (OriginBall :type "Array of Integer"))
  (returns (SortedBall :type "Array of Integer"))
  (locals (LOriginBall :type "Array of Integer") (LLength :type Integer) (LReturnBall :type "Array of Integer"))
  (bind _loriginball (`local.LOriginBall`))
  (bind (_indexofminvalue _minvalue) (`KismetMathLibrary.MinOfIntArray` _loriginball))
  (bind _output_get (set `local.LOriginBall` OriginBall))
  (bind _output_get_2 (set `local.LLength` (`KismetArrayLibrary.Array_Length` _output_get)))
  (for _ (range _output_get_2)
    (`KismetArrayLibrary.Array_Add` (`local.LReturnBall`) _minvalue)
    (`KismetArrayLibrary.Array_Remove` _loriginball _indexofminvalue))
  (return (`local.LReturnBall`)))

(fn `UpdateBallNums`
  (params (BallNumType :type "/Game/Blueprints/EnumBallNumType Enum" :default "NewEnumerator0") (BallNum :type Integer))
  (locals (LNum :type Integer) (LNum :type Integer))
  (bind _lnum (`local.LNum`))
  (set `local.LNum` BallNum)
  (switch `/Game/Blueprints/EnumBallNumType` BallNumType
    (:`NewEnumerator0`
      (set `self.RedBallTotal` _lnum))
    (:`NewEnumerator1`
      (set `self.RedBallChoose` _lnum))
    (:`NewEnumerator2`
      (set `self.BlueBallTotal` _lnum))
    (:`NewEnumerator3`
      (set `self.BlueBallChoose` _lnum))))

(fn `UserConstructionScript`)

(fn `WhetherWinPrice`
  (params (ChampionType :type "/Game/Blueprints/ChampionType Enum" :default "NewEnumerator0") (ExpectPrice :type Integer) (Results :type "Array of Integer"))
  (returns (WhetherPrice :type Boolean) (PriceLevel :type Integer) (PositionResult :type "Array of Boolean") (HitRedNum :type Integer) (HitBlueNum :type Integer))
  (locals (LChampionType :type "/Game/Blueprints/ChampionType Enum") (LExpectPrice :type Integer) (LSimulateNumbers :type "Array of Integer") (LNo1PriceNumbers :type "Array of Integer"))
  (set `local.LChampionType` ChampionType)
  (set `local.LExpectPrice` ExpectPrice)
  (set `local.LSimulateNumbers` Results)
  (bind _outnumbers (`/Game/UI/WB_MainColorPanle.GetPriceNumbers` (`self.PanelVaria`)))
  (set `local.LNo1PriceNumbers` _outnumbers)
  (switch `/Game/Blueprints/ChampionType` ChampionType
    (:`NewEnumerator0`
      (bind (_redtimes _bluetiems _positionresult) (`self.CheckHowMuchBallHit` (`local.LSimulateNumbers`) (`local.LNo1PriceNumbers`)))
      (bind _winpricelevel (`self.CheckWinPriceLevelByExpect_DLT` (`local.LExpectPrice`) _redtimes _bluetiems))
      (return (> _winpricelevel 0) _winpricelevel _positionresult _redtimes _bluetiems))
    (:`NewEnumerator1`
      (bind (_redtimes_2 _bluetiems_2 _positionresult_2) (`self.CheckHowMuchBallHit` (`local.LSimulateNumbers`) (`local.LNo1PriceNumbers`) "NewEnumerator1"))
      (bind _winpricelevel_2 (`self.CheckWinPriceLevelByExpect_SSQ` (`local.LExpectPrice`) _redtimes_2 _bluetiems_2))
      (return (> _winpricelevel_2 0) _winpricelevel_2 _positionresult_2 _redtimes_2 _bluetiems_2))))